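; BP_Player is the player Blueprint for a bowling game, handling aim and a one-shot throw of the ball.
; The mouse wheel yaws an Arrow component to set the throw direction.
; Left click, gated by a DoOnce, enables physics on BowlingBall and applies an impulse along the arrow's forward vector scaled by ThrowSpeed.
; Right click calls OpenLevelByName with the name None, then resets the DoOnce.
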(event `InputAxisKey|MouseWheelAxis`
  (params (AxisValue :type "Float (single-precision)"))
  (`SceneComponent.K2_AddLocalRotation` (`self.Arrow`) (`KismetMathLibrary.MakeRotator` 0.0 0.0 AxisValue) false false))

(event `Key|LeftMouseButton`
  (params (Key :type "Key Structure"))
  (bind _bowlingball (`self.BowlingBall`))
  (:`Pressed`
    (`/Engine/EditorBlueprintResources/StandardMacros.DoOnce` false :!label _label
      (:`Completed`
        (`PrimitiveComponent.SetSimulatePhysics` _bowlingball true)
        (`PrimitiveComponent.AddImpulse` _bowlingball (* (`SceneComponent.GetForwardVector` (`self.Arrow`)) (`self.Throw Speed`)) "None" false)))))

(event `Key|RightMouseButton`
  (params (Key :type "Key Structure"))
  (:`Pressed`
    (`GameplayStatics.OpenLevel` "None")
    (goto _label :!via `Reset`)))

(fn `UserConstructionScript`)